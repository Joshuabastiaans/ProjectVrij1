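; BP_RecieveWood is a stove fuel receiver, hidden at BeginPlay, that shows itself while wood burns.
; FireInStove plays a refill sound chosen by an incrementing index, triggers fire-stoke audio, and sets active fuel on A_ShipPos.
; A retriggerable delay of FuelTimer restarts with each call; on expiry it stops the fire sound, hides the actor and clears active fuel.
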(event `PlaySound`
  (bind _bijvullen2 (`self.Bijvullen2`))
  (bind _bijvullen1 (`self.Bijvullen1`))
  (if (`self.CanPlay`)
    (if (== (`self.WhichSound`) 0)
      (`AudioParameterControllerInterface.SetTriggerParameter` _bijvullen1 "Play")
      (`AudioComponent.SetWaveParameter` _bijvullen1 "Name" "/Game/Sound/Internal_Dialogue/FuelBijvullen1.FuelBijvullen1")
      (`AudioParameterControllerInterface.SetFloatParameter` _bijvullen1 "Gain" 2.0)
      (elif (== (`self.WhichSound`) 1)
        (`AudioParameterControllerInterface.SetTriggerParameter` _bijvullen2 "Play")
        (`AudioComponent.SetWaveParameter` _bijvullen2 "Name" "/Game/Sound/Internal_Dialogue/FuelBijvullen1.FuelBijvullen1")
        (`AudioParameterControllerInterface.SetFloatParameter` _bijvullen2 "Gain" 2.0)))))

(event `self.ReceiveBeginPlay`
  (`self.SetActorHiddenInGame` true))

(event `FireInStove`
  ;[1 1 1] FireInStove
  (`|ExecutionSequence`
    (:`then_0`
      (`self.PlaySound`)
      (bind _output_get (set `self.WhichSound` (+ (stale _output_get) 1)))
      (`AudioParameterControllerInterface.SetTriggerParameter` (`self.FireSound`) "FireStoke")
      (`KismetSystemLibrary.RetriggerableDelay` (`self.FuelTimer`))
      (`AudioParameterControllerInterface.SetTriggerParameter` (`self.FireSound`) "Stop")
      (`self.SetActorHiddenInGame` true)
      (bind _returnvalue (`GameplayStatics.GetActorOfClass` "/Game/ShipNav/A_ShipPos.A_ShipPos_C"))
      (`/Game/ShipNav/A_ShipPos.SetActiveFuel` _returnvalue false))
    (:`then_1`
      (`self.SetActorHiddenInGame` false)
      (bind _returnvalue_2 (`GameplayStatics.GetActorOfClass` "/Game/ShipNav/A_ShipPos.A_ShipPos_C"))
      (`/Game/ShipNav/A_ShipPos.SetActiveFuel` _returnvalue_2 true))))

(event `self.ReceiveTick`
  (params (DeltaSeconds :type "Float (single-precision)")))

(fn `UserConstructionScript`)
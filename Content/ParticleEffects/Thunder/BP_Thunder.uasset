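; BP_Thunder is a recurring thunder effect that plays a sound and animates a ThunderPlane through its material.
; BeginPlay starts an endless loop that waits a random 20 to 80 seconds, then calls the Thunder event.
; When IsThunder is set, that event fires the audio's Play trigger and restarts a timeline whose curve drives the plane's Y and emission material parameters.
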(event `Thunder`
  (bind _thunderplane (`self.ThunderPlane`))
  (if (`self.IsThunder`)
    (`AudioParameterControllerInterface.SetTriggerParameter` (`self.ThunderAudio`) "Play")
    (bind (_direction _timeline) (`Timeline|ThunderTL` :!via `PlayFromStart`)
      (:`Update`
        (`MeshComponent.SetScalarParameterValueOnMaterials` _thunderplane "Y" _timeline)
        (`MeshComponent.SetScalarParameterValueOnMaterials` _thunderplane "Emmision" (* (+ _timeline 1.0) 20.0))))))

(event `self.ReceiveBeginPlay`
  (`KismetSystemLibrary.Delay` (`KismetMathLibrary.RandomFloatInRange` 20.0 80.0) :!label _label)
  (`self.Thunder`)
  (goto _label))

(fn `UserConstructionScript`)
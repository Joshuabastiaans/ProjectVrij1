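; Event manager for the ship navigation game that runs a timed opening sequence from tutorial to storm.
; On BeginPlay it hides itself, waits, plays the tutorial voice line, then sends IsCycling to the level once the line's duration has passed.
; After a longer delay it unhides itself, flags every BP_Thunder actor as thundering and starts rain audio through parameter-driven audio components.
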(event `self.ReceiveBeginPlay`
  (bind _playaudio (`self.PlayAudio`))
  (bind _rainaudio (`self.RainAudio`))
  (`self.SetActorHiddenInGame` true)
  (`KismetSystemLibrary.Delay` 15.0)
  (`AudioComponent.SetWaveParameter` _playaudio "Name" "/Game/Sound/Internal_Dialogue/Tutorial_Aanwijzing.Tutorial_Aanwijzing")
  (`AudioParameterControllerInterface.SetTriggerParameter` _playaudio "Play")
  (`KismetSystemLibrary.Delay` (`self.VoiceLineDuration`))
  (message `AudioParameterControllerInterface.SetBoolParameter` (`self.GetLevel`) "IsCycling" true)
  (`KismetSystemLibrary.Delay` 100.0)
  (`self.SetActorHiddenInGame` false)
  (bind _outactors (`GameplayStatics.GetAllActorsOfClass` "/Game/ParticleEffects/Thunder/BP_Thunder.BP_Thunder_C"))
  (for _array_element _outactors
    (set `/Game/ParticleEffects/Thunder/BP_Thunder.IsThunder` true _array_element))
  (`AudioParameterControllerInterface.SetTriggerParameter` _rainaudio "Play")
  (`AudioComponent.SetWaveParameter` _rainaudio "Name" "/Game/Sound/Rain.Rain")
  (`AudioParameterControllerInterface.SetFloatParameter` _rainaudio "Gain" 0.5))

(fn `UserConstructionScript`)
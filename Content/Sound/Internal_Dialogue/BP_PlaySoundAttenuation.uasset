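; Actor Blueprint that plays a configurable sound through its PlayAudio component after a delay once play begins.
; On BeginPlay it passes the audio file, loop flag and gain to the sound as named parameters, waits, then fires the Play trigger.
; Immediately afterwards it finds the BP_PlayRadioMusic actor in the level and calls ChangePitch on it.
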(event `self.ReceiveBeginPlay`
  (bind _playaudio (`self.PlayAudio`))
  (`AudioComponent.SetWaveParameter` _playaudio "Name" (`self.AudioFile`))
  (`AudioParameterControllerInterface.SetBoolParameter` _playaudio "Loop" (`self.Loop`))
  (`AudioParameterControllerInterface.SetFloatParameter` _playaudio "Gain" (`self.Gain`))
  (`KismetSystemLibrary.Delay` (`self.Delay`))
  (`AudioParameterControllerInterface.SetTriggerParameter` _playaudio "Play")
  (bind _returnvalue (`GameplayStatics.GetActorOfClass` "/Game/Sound/BP_PlayRadioMusic.BP_PlayRadioMusic_C"))
  (`/Game/Sound/BP_PlayRadioMusic.ChangePitch` _returnvalue))

(fn `UserConstructionScript`)